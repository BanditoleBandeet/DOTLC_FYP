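; Parent Blueprint for a harvestable tree resource that takes damage until it is destroyed and can leave a stump behind.
; BeginPlay caches the stump spawn component's world transform, and AnyDamage subtracts from Health with a debug print.
; At zero health it spawns a stump if its display name contains "ResourceTree", then destroys itself.
; Nodes for controller action state and delayed physics despawn are unconnected.
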(event `self.ReceiveBeginPlay`
  (`parent.ReceiveBeginPlay`)
  (set `self.StumpTransform` (`SceneComponent.K2_GetComponentToWorld` (`self.StumpSpawnLocation`))))

(event `self.ReceiveAnyDamage`
  (params (Damage :type "Float (single-precision)") (DamageType :type "DamageType Object Reference") (InstigatedBy :type "Controller Object Reference") (DamageCauser :type "Actor Object Reference"))
  (bind _output_get (set `self.Health` (- (`self.Health`) Damage)))
  ;[1 0 0.5802] PRINT STRING
  (`KismetSystemLibrary.PrintString` (`KismetStringLibrary.Concat_StrStr` "Resource Health = " (`KismetStringLibrary.Conv_DoubleToString` _output_get)) true true (struct :`R` 0.057249 :`G` 1.0 :`A` 1.0))
  (if (<= _output_get 0.0)
    (if (`KismetStringLibrary.Contains` (`KismetSystemLibrary.GetDisplayName` self) "ResourceTree")
      (`|SpawnActorFromClass` "/Game/Resources/Tree/BP_StumpResourceTree01.BP_StumpResourceTree01_C" (`self.StumpTransform`) "AdjustIfPossibleButAlwaysSpawn" "OverrideRootScale" null null))
    (`self.K2_DestroyActor`)))

(fn `UserConstructionScript`
  (`parent.UserConstructionScript`))