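; Tier 1 Herbalist building that is meant to supply the colony with medicine on a timer.
; On BeginPlay it runs parent logic, checks for the top-down game mode and starts a looping 15-second AddMedicineHourly timer.
; That event adds one resource unit through AddResourceValue, but a DoOnce with no reset limits it to the first firing.
; A colony resource modifier increment is left unconnected.
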(event `self.ReceiveBeginPlay`
  (`parent.ReceiveBeginPlay`)
  (bind _asbp_gm_top_down_game_mode (cast `/Game/Blueprints/Gamemodes/BP_GM_TopDownGameMode` (`GameplayStatics.GetGameMode`)))
  (`KismetSystemLibrary.K2_SetTimerDelegate` (delegate `AddMedicineHourly`) 15.0 true))

(event `AddMedicineHourly`
  (`/Engine/EditorBlueprintResources/StandardMacros.DoOnce` false
    (:`Completed`
      (`/Game/Blueprints/Function_Libraries/FL_ResourceInteractions.Add Resource Value` 1 "NewEnumerator3"))))

(fn `UserConstructionScript`
  (`parent.UserConstructionScript`))