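; BP_GuardTower is a guard tower building Blueprint that responds to left mouse clicks.
; On click, it clears the friendly selection on the top-down survivor controller, then runs the parent click handler.
; It then sets the camera location to the tower through its SurvivorControllerREF reference.
; The construction script only calls the parent's.
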(event `self.ReceiveActorOnClicked`
  (params (ButtonPressed :type "Key Structure"))
  (if (== ButtonPressed "LeftMouseButton")
    (bind _asbp_top_down_survivor_controller (cast `/Game/Blueprints/Controllers/BP_TopDownSurvivorController` (`GameplayStatics.GetPlayerController` 0)))
    (`/Game/Blueprints/Controllers/BP_TopDownSurvivorController.ClearFriendlySelection` _asbp_top_down_survivor_controller)
    (`parent.ReceiveActorOnClicked` ButtonPressed)
    (`/Game/Blueprints/Controllers/BP_TopDownSurvivorController.SetCameraLocation` (`self.SurvivorControllerREF`) (`self.K2_GetActorLocation`))))

(fn `UserConstructionScript`
  (`parent.UserConstructionScript`))