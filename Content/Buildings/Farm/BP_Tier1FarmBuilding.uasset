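; Tier 1 farm building that raises the colony's food per hour, built on a parent building class.
; AddFoodPerHour adds a fixed amount to the food entry in the game mode's ColonyResourceModifierMap.
; That event is bound to the AddFoodPerHour dispatcher on every Tick rather than once at BeginPlay.
; A left click clears the player controller's friendly selection before running the parent click logic, and GetHoverWidget returns nothing.
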(event `self.ReceiveBeginPlay`
  (`parent.ReceiveBeginPlay`))

(event `AddFoodPerHour`
  (bind _asbp_gm_top_down_game_mode (cast `/Game/Blueprints/Gamemodes/BP_GM_TopDownGameMode` (`GameplayStatics.GetGameMode`)))
  (bind _colonyresourcemodifiermap (`/Game/Blueprints/Gamemodes/BP_GM_TopDownGameMode.ColonyResourceModifierMap` _asbp_gm_top_down_game_mode))
  (`BlueprintMapLibrary.Map_Add` _colonyresourcemodifiermap "NewEnumerator3" (+ (`BlueprintMapLibrary.Map_Find` _colonyresourcemodifiermap "NewEnumerator3") 2))
  (set `/Game/Blueprints/Gamemodes/BP_GM_TopDownGameMode.ColonyResourceModifierMap` _colonyresourcemodifiermap _asbp_gm_top_down_game_mode))

(event `self.ReceiveTick`
  (params (DeltaSeconds :type "Float (single-precision)"))
  (`parent.ReceiveTick` DeltaSeconds)
  (`/Engine/EditorBlueprintResources/StandardMacros.IsValid` self
    (:`Is Valid`
      (add `self.EventDispatcherAddFoodPerHour` (delegate `AddFoodPerHour`)))))

(event `self.ReceiveActorOnClicked`
  (params (ButtonPressed :type "Key Structure"))
  (if (== ButtonPressed "LeftMouseButton")
    (bind _asbp_top_down_survivor_controller (cast `/Game/Blueprints/Controllers/BP_TopDownSurvivorController` (`GameplayStatics.GetPlayerController` 0)))
    (`/Game/Blueprints/Controllers/BP_TopDownSurvivorController.ClearFriendlySelection` _asbp_top_down_survivor_controller)
    (`parent.ReceiveActorOnClicked` ButtonPressed)))

(fn `GetHoverWidget`
  (returns (Widget :type "WidgetComponent Object Reference"))
  (return null))

(fn `UserConstructionScript`
  (`parent.UserConstructionScript`))