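; BP_Tier1House is the tier 1 house building, a child Blueprint that adds click handling to its parent's behavior.
; On a left click it casts the player controller to BP_TopDownSurvivorController, clears the friendly selection, then calls the parent's click handler.
; Other mouse buttons or a failed cast skip the parent handler entirely.
; The construction script only calls the parent, and BeginPlay, overlap and Tick are unused.
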(event `self.ReceiveActorOnClicked`
  (params (ButtonPressed :type "Key Structure"))
  (if (== ButtonPressed "LeftMouseButton")
    (bind _asbp_top_down_survivor_controller (cast `/Game/Blueprints/Controllers/BP_TopDownSurvivorController` (`GameplayStatics.GetPlayerController` 0)))
    (`/Game/Blueprints/Controllers/BP_TopDownSurvivorController.ClearFriendlySelection` _asbp_top_down_survivor_controller)
    (`parent.ReceiveActorOnClicked` ButtonPressed)))

(fn `UserConstructionScript`
  (`parent.UserConstructionScript`))