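; Blueprint function library for reading and adjusting stats on the player's survivor character.
; Each function casts player character 0 to BP_SurvivorMainCharacter and works on its Stats map by key.
; Add and Minus write the current value plus or minus an amount back to the map without clamping, while Get returns the stored value.
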(fn `Add Main Character Stat Value`
  (params (`Stat to Minus` :type "/Game/Enums/E_ColonyStatTypes Enum" :default "NewEnumerator0") (`Amount to Minus` :type "Float (double-precision)"))
  (bind _asbp_survivor_main_character (cast `/Game/Blueprints/BP_SurvivorMainCharacter` (`GameplayStatics.GetPlayerCharacter` null)))
  (bind _stats (`/Game/Blueprints/BP_SurvivorMainCharacter.Stats` _asbp_survivor_main_character))
  (`BlueprintMapLibrary.Map_Add` _stats `Stat to Minus` (+ (`BlueprintMapLibrary.Map_Find` _stats `Stat to Minus`) `Amount to Minus`)))

(fn `Get Main Character Stat Value`
  (params (Stat :type "/Game/Enums/E_ColonyStatTypes Enum" :default "NewEnumerator0"))
  (returns (Value :type "Float (double-precision)"))
  (bind _asbp_survivor_main_character (cast `/Game/Blueprints/BP_SurvivorMainCharacter` (`GameplayStatics.GetPlayerCharacter` null)))
  (return (`BlueprintMapLibrary.Map_Find` (`/Game/Blueprints/BP_SurvivorMainCharacter.Stats` _asbp_survivor_main_character) Stat)))

(fn `Minus Main Character Stat Value`
  (params (`Stat to Minus` :type "/Game/Enums/E_ColonyStatTypes Enum" :default "NewEnumerator0") (`Amount to Minus` :type "Float (double-precision)"))
  (bind _asbp_survivor_main_character (cast `/Game/Blueprints/BP_SurvivorMainCharacter` (`GameplayStatics.GetPlayerCharacter` null)))
  (bind _stats (`/Game/Blueprints/BP_SurvivorMainCharacter.Stats` _asbp_survivor_main_character))
  (`BlueprintMapLibrary.Map_Add` _stats `Stat to Minus` (- (`BlueprintMapLibrary.Map_Find` _stats `Stat to Minus`) `Amount to Minus`)))