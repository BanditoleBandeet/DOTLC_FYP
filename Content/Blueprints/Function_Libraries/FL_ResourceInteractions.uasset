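; Blueprint function library for reading and changing the colony's resource totals, Wood and Scrap.
; Each function casts the game mode to BP_GM_TopDownGameMode and works on its ColonyResourceModifierMap, keyed by resource type.
; Add and Minus switch on the type, write the adjusted value back without any clamping, and Get returns the stored value for the given type.
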(fn `Add Resource Value`
  (params (`Amount To Add` :type Integer) (ResourceType :type "/Game/Enums/E_ResourceTypes Enum" :default "NewEnumerator0"))
  (returns (ResourceGatherType :type "/Game/Enums/E_ResourceTypes Enum"))
  (locals (`Amount to Add to Resources` :type Integer))
  (bind _output_get (set `local.Amount to Add to Resources` `Amount To Add`))
  (bind _asbp_gm_top_down_game_mode (cast `/Game/Blueprints/Gamemodes/BP_GM_TopDownGameMode` (`GameplayStatics.GetGameMode` null)))
  (switch `/Game/Enums/E_ResourceTypes` ResourceType
    (:`NewEnumerator0`
      (bind _colonyresourcemodifiermap (`/Game/Blueprints/Gamemodes/BP_GM_TopDownGameMode.ColonyResourceModifierMap` _asbp_gm_top_down_game_mode))
      (`BlueprintMapLibrary.Map_Add` _colonyresourcemodifiermap "NewEnumerator1" (+ (`BlueprintMapLibrary.Map_Find` _colonyresourcemodifiermap "NewEnumerator1") _output_get))
      (set `/Game/Blueprints/Gamemodes/BP_GM_TopDownGameMode.ColonyResourceModifierMap` _colonyresourcemodifiermap _asbp_gm_top_down_game_mode))
    (:`NewEnumerator1`
      (`BlueprintMapLibrary.Map_Add` _colonyresourcemodifiermap "NewEnumerator0" (+ (`BlueprintMapLibrary.Map_Find` _colonyresourcemodifiermap "NewEnumerator0") _output_get))
      (set `/Game/Blueprints/Gamemodes/BP_GM_TopDownGameMode.ColonyResourceModifierMap` _colonyresourcemodifiermap _asbp_gm_top_down_game_mode)))
  (return ResourceType))

(fn `Get Resource Stat Value`
  (params (`Resource Type` :type "/Game/Enums/E_Resources Enum" :default "NewEnumerator0"))
  (returns (Value :type Integer))
  (bind _asbp_gm_top_down_game_mode (cast `/Game/Blueprints/Gamemodes/BP_GM_TopDownGameMode` (`GameplayStatics.GetGameMode` null)))
  (return (`BlueprintMapLibrary.Map_Find` (`/Game/Blueprints/Gamemodes/BP_GM_TopDownGameMode.ColonyResourceModifierMap` _asbp_gm_top_down_game_mode) `Resource Type`)))

(fn `Minus Resource Stat Value`
  (params (`Amount To Minus` :type Integer) (ResourceType :type "/Game/Enums/E_ResourceTypes Enum" :default "NewEnumerator0"))
  (locals (`Amount to Minus From Resources` :type Integer))
  (set `local.Amount to Minus From Resources` `Amount To Minus`)
  (bind _asbp_gm_top_down_game_mode (cast `/Game/Blueprints/Gamemodes/BP_GM_TopDownGameMode` (`GameplayStatics.GetGameMode` null)))
  (switch `/Game/Enums/E_ResourceTypes` ResourceType
    (:`NewEnumerator0`
      (bind _colonyresourcemodifiermap (`/Game/Blueprints/Gamemodes/BP_GM_TopDownGameMode.ColonyResourceModifierMap` _asbp_gm_top_down_game_mode))
      (`BlueprintMapLibrary.Map_Add` _colonyresourcemodifiermap "NewEnumerator1" (- (`BlueprintMapLibrary.Map_Find` _colonyresourcemodifiermap "NewEnumerator1") (`local.Amount to Minus From Resources`)))
      (set `/Game/Blueprints/Gamemodes/BP_GM_TopDownGameMode.ColonyResourceModifierMap` _colonyresourcemodifiermap _asbp_gm_top_down_game_mode))
    (:`NewEnumerator1`
      (`BlueprintMapLibrary.Map_Add` _colonyresourcemodifiermap "NewEnumerator0" (- (`BlueprintMapLibrary.Map_Find` _colonyresourcemodifiermap "NewEnumerator0") (`local.Amount to Minus From Resources`)))
      (set `/Game/Blueprints/Gamemodes/BP_GM_TopDownGameMode.ColonyResourceModifierMap` _colonyresourcemodifiermap _asbp_gm_top_down_game_mode))))