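; Blueprint function library for reading, increasing and decreasing the stats of the player's FriendlyAIChild character.
; Each function casts player character 0 to FriendlyAIChild, so it only takes effect when the player is that class.
; Stats live in the FriendlyAIStats map; changes find the current value, apply the amount and write it back under the same key, with no clamping.
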(fn `Add Friendly AI Stat Value`
  (params (`Stat to Minus` :type "/Game/Enums/E_ColonyStatTypes Enum" :default "NewEnumerator0") (`Amount to Minus` :type "Float (double-precision)") (__WorldContext :type "Object Object Reference"))
  (bind _asfriendly_aichild (cast `/Game/FriendlyAI/FriendlyAIChild` (`GameplayStatics.GetPlayerCharacter` __WorldContext)))
  (bind _friendlyaistats (`/Game/FriendlyAI/ParentClass/FriendlyAI_Parent.FriendlyAIStats` _asfriendly_aichild))
  (`BlueprintMapLibrary.Map_Add` _friendlyaistats `Stat to Minus` (+ (`BlueprintMapLibrary.Map_Find` _friendlyaistats `Stat to Minus`) `Amount to Minus`)))

(fn `Get Friendly AI Stat Value`
  (params (Stat :type "/Game/Enums/E_ColonyStatTypes Enum" :default "NewEnumerator0") (__WorldContext :type "Object Object Reference"))
  (returns (Value :type "Float (double-precision)"))
  (bind _asfriendly_aichild (cast `/Game/FriendlyAI/FriendlyAIChild` (`GameplayStatics.GetPlayerCharacter` __WorldContext)))
  (return (`BlueprintMapLibrary.Map_Find` (`/Game/FriendlyAI/ParentClass/FriendlyAI_Parent.FriendlyAIStats` _asfriendly_aichild) Stat)))

(fn `Minus Friendly AI Stat Value`
  (params (`Stat to Minus` :type "/Game/Enums/E_ColonyStatTypes Enum" :default "NewEnumerator0") (`Amount to Minus` :type "Float (double-precision)") (__WorldContext :type "Object Object Reference"))
  (bind _asfriendly_aichild (cast `/Game/FriendlyAI/FriendlyAIChild` (`GameplayStatics.GetPlayerCharacter` __WorldContext)))
  (bind _friendlyaistats (`/Game/FriendlyAI/ParentClass/FriendlyAI_Parent.FriendlyAIStats` _asfriendly_aichild))
  (`BlueprintMapLibrary.Map_Add` _friendlyaistats `Stat to Minus` (- (`BlueprintMapLibrary.Map_Find` _friendlyaistats `Stat to Minus`) `Amount to Minus`)))