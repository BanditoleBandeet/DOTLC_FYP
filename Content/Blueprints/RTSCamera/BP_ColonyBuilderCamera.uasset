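; Colony-builder RTS camera actor that blends in as the player's view on BeginPlay and edge-scrolls with the mouse.
; Each Tick, four checks scale CameraSpeed by cursor depth into thin viewport-edge bands and offset the root.
; As written, opposite edges add same-sign offsets.
; Increase/decrease functions multiply four directional speed variables, which the movement checks never read.
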(event `self.ReceiveBeginPlay`
  (`self.Set Colony Build Mode Camera`))

(event `self.ReceiveTick`
  (params (DeltaSeconds :type "Float (single-precision)"))
  (`self.CameraMoveLeftCheck`)
  (`self.CameraMoveRightCheck`)
  (`self.CameraMoveUpCheck`)
  (`self.CameraMoveDownCheck`))

(fn `CameraMoveDownCheck`
  (locals (`Camera Speed` :type "Float (double-precision)" :default -75.0))
  (bind (_returnvalue_x _returnvalue_y) (`KismetMathLibrary.BreakVector2D` (`WidgetLayoutLibrary.GetViewportSize`)))
  (bind _returnvalue (`WidgetLayoutLibrary.GetMousePositionOnViewport`))
  (bind (_returnvalue_x_2 _returnvalue_y_2) (`KismetMathLibrary.BreakVector2D` (* _returnvalue (`WidgetLayoutLibrary.GetViewportScale`))))
  (`SceneComponent.K2_AddRelativeLocation` (`self.DefaultSceneRoot`) (* (`KismetMathLibrary.MakeVector` 0.0 (`local.Camera Speed`)) (`KismetMathLibrary.FClamp` (`KismetMathLibrary.NormalizeToRange` _returnvalue_y_2 (* _returnvalue_y 0.99) _returnvalue_y))) false false))

(fn `CameraMoveLeftCheck`
  (locals (CameraSpeed :type "Float (double-precision)" :default 100.0))
  (bind _returnvalue_x (`KismetMathLibrary.BreakVector2D` (`WidgetLayoutLibrary.GetViewportSize`)))
  (bind _returnvalue (`WidgetLayoutLibrary.GetMousePositionOnViewport`))
  (bind _returnvalue_x_2 (`KismetMathLibrary.BreakVector2D` (* _returnvalue (`WidgetLayoutLibrary.GetViewportScale`))))
  (`SceneComponent.K2_AddRelativeLocation` (`self.DefaultSceneRoot`) (* (`KismetMathLibrary.MakeVector` (`local.CameraSpeed`)) (- 1.0 (`KismetMathLibrary.FClamp` (`KismetMathLibrary.NormalizeToRange` _returnvalue_x_2 0.0 (* _returnvalue_x 0.01))))) false false))

(fn `CameraMoveRightCheck`
  (locals (`Camera Speed` :type "Float (double-precision)" :default -100.0))
  (bind _returnvalue_x (`KismetMathLibrary.BreakVector2D` (`WidgetLayoutLibrary.GetViewportSize`)))
  (bind _returnvalue (`WidgetLayoutLibrary.GetMousePositionOnViewport`))
  (bind _returnvalue_x_2 (`KismetMathLibrary.BreakVector2D` (* _returnvalue (`WidgetLayoutLibrary.GetViewportScale`))))
  (`SceneComponent.K2_AddRelativeLocation` (`self.DefaultSceneRoot`) (* (`KismetMathLibrary.MakeVector` (`local.Camera Speed`)) (`KismetMathLibrary.FClamp` (`KismetMathLibrary.NormalizeToRange` _returnvalue_x_2 (* _returnvalue_x 0.99) _returnvalue_x))) false false))

(fn `CameraMoveUpCheck`
  (locals (`Camera Speed` :type "Float (double-precision)" :default 75.0))
  (bind (_returnvalue_x _returnvalue_y) (`KismetMathLibrary.BreakVector2D` (`WidgetLayoutLibrary.GetViewportSize`)))
  (bind _returnvalue (`WidgetLayoutLibrary.GetMousePositionOnViewport`))
  (bind (_returnvalue_x_2 _returnvalue_y_2) (`KismetMathLibrary.BreakVector2D` (* _returnvalue (`WidgetLayoutLibrary.GetViewportScale`))))
  (`SceneComponent.K2_AddRelativeLocation` (`self.DefaultSceneRoot`) (* (`KismetMathLibrary.MakeVector` 0.0 (`local.Camera Speed`)) (- 1.0 (`KismetMathLibrary.FClamp` (`KismetMathLibrary.NormalizeToRange` _returnvalue_y_2 0.0 (* _returnvalue_y 0.01))))) false false))

(fn `DecreaseCameraSpeed`
  (params (CameraMovementSpeedReductionMultiplier :type "Float (double-precision)"))
  (returns (`Decreased Left Movement Speed` :type "Float (double-precision)") (`Decreased Up Movement Speed` :type "Float (double-precision)") (`Decreased Down Movement Speed` :type "Float (double-precision)") (`Decreased Right Movement Speed` :type "Float (double-precision)"))
  (bind _cameramovementspeedreductionmultiplier (`self.CameraMovementSpeedReductionMultiplier`))
  (set `self.CameraMovementSpeedReductionMultiplier` CameraMovementSpeedReductionMultiplier)
  (bind _output_get (set `self.Left Movement Speed` (* (`self.Left Movement Speed`) _cameramovementspeedreductionmultiplier)))
  (bind _output_get_2 (set `self.UpMovementSpeed` (* (`self.UpMovementSpeed`) _cameramovementspeedreductionmultiplier)))
  (bind _output_get_3 (set `self.DownMovementSpeed` (* (`self.DownMovementSpeed`) _cameramovementspeedreductionmultiplier)))
  (bind _output_get_4 (set `self.Right Movement Speed` (* (`self.Right Movement Speed`) _cameramovementspeedreductionmultiplier)))
  (return _output_get _output_get_2 _output_get_3 _output_get_4))

(fn `IncreaseCameraSpeed`
  (params (CameraMovementSpeedMultiplier :type "Float (double-precision)"))
  (returns (`Increased Left Movement Speed` :type "Float (double-precision)") (`Increased Up Movement Speed` :type "Float (double-precision)") (`Increased Down Movement Speed` :type "Float (double-precision)") (`Increased Right Movement Speed` :type "Float (double-precision)"))
  (bind _cameramovementspeedmultiplier (`self.CameraMovementSpeedMultiplier`))
  (set `self.CameraMovementSpeedMultiplier` CameraMovementSpeedMultiplier)
  (bind _output_get (set `self.Left Movement Speed` (* (`self.Left Movement Speed`) _cameramovementspeedmultiplier)))
  (bind _output_get_2 (set `self.UpMovementSpeed` (* (`self.UpMovementSpeed`) _cameramovementspeedmultiplier)))
  (bind _output_get_3 (set `self.DownMovementSpeed` (* (`self.DownMovementSpeed`) _cameramovementspeedmultiplier)))
  (bind _output_get_4 (set `self.Right Movement Speed` (* (`self.Right Movement Speed`) _cameramovementspeedmultiplier)))
  (return _output_get _output_get_2 _output_get_3 _output_get_4))

(fn `Set Colony Build Mode Camera`
  (`PlayerController.SetViewTargetWithBlend` (`GameplayStatics.GetPlayerController` 0) self 5.0 "VTBlend_Linear" 0.5 false))

(fn `UserConstructionScript`)