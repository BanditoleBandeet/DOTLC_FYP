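; Zombie spawner actor that runs SpawnZombies on a looping timer, placing ZombieAI at random navigable points near SpawnLocation.
; SpawnZombies switches on CurrentMaxZombiesToSpawn to pick a per-day interval, then adds the game mode's days survived to that count.
; Its loop spawns only when the index equals the count and otherwise calls a break.
; The timer is set once at BeginPlay, so later interval changes never reach it.
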(event `self.ReceiveBeginPlay`
  (bind _asbp_gm_top_down_game_mode (cast `/Game/Blueprints/Gamemodes/BP_GM_TopDownGameMode` (`GameplayStatics.GetGameMode`)))
  (set `self.Top Down Game Mode_REF` _asbp_gm_top_down_game_mode)
  (set `self.CurrentMaxZombiesToSpawn` (`self.CurrentMaxZombiesToSpawn`))
  (set `self.SpawnTransform` (`KismetMathLibrary.MakeTransform` (`SceneComponent.K2_GetComponentLocation` (`self.SpawnLocation`)) (`SceneComponent.K2_GetComponentRotation` (`self.SpawnRotationDirection`))))
  (`KismetSystemLibrary.K2_SetTimerDelegate` (delegate `SpawnZombies`) (`self.DefaultSpawnerTimer`) true))

(event `SpawnZombies`
  (bind (_spawntransform_location _spawntransform_rotation) (`KismetMathLibrary.BreakTransform` (`self.SpawnTransform`)))
  (bind _currentmaxzombiestospawn (`self.CurrentMaxZombiesToSpawn`))
  (switch `int` _currentmaxzombiestospawn
    (:`1`
      (set `self.DefaultSpawnerTimer` (`self.Day1ZombieSpawnTimeInterval`)))
    (:`2`
      (set `self.DefaultSpawnerTimer` (`self.Day2ZombieSpawnTimeInterval`)))
    (:`3`
      (set `self.DefaultSpawnerTimer` (`self.Day3ZombieSpawnTimeInterval`)))
    (:`4`
      (set `self.DefaultSpawnerTimer` (`self.Day4ZombieSpawnTimeInterval`)))
    (:`5`
      (set `self.DefaultSpawnerTimer` (`self.Day5ZombieSpawnTimeInterval`)))
    (:`6`
      (set `self.DefaultSpawnerTimer` (`self.Day6ZombieSpawnTimeInterval`)))
    (:`7`
      (set `self.DefaultSpawnerTimer` (`self.Day7ZombieSpawnTimeInterval`))))
  (set `self.CurrentMaxZombiesToSpawn` (+ _currentmaxzombiestospawn (`/Game/Blueprints/Gamemodes/BP_GM_TopDownGameMode.CurrentDaysSurvived` (`self.Top Down Game Mode_REF`))))
  (for _index (range (+ (`self.CurrentMaxZombiesToSpawn`) 1)) :!label _label
    (if (== _index (`self.CurrentMaxZombiesToSpawn`))
      (bind _randomlocation (`NavigationSystemV1.K2_GetRandomLocationInNavigableRadius` _spawntransform_location 100.0 null null))
      (bind _returnvalue (`|SpawnActorFromClass` "/Game/ZombieAI/ZombieAI.ZombieAI_C" (`KismetMathLibrary.Conv_VectorToTransform` _randomlocation) "AdjustIfPossibleButAlwaysSpawn" "OverrideRootScale" null null))
      (`self.K2_SetActorRotation` _returnvalue _spawntransform_rotation false)
      (`/Engine/EditorBlueprintResources/StandardMacros.IncrementInt` _index)
      (else
        (`self.BreakZombieSpawnLoop`)))))

(event `BreakZombieSpawnLoop`
  (goto _label :!via `Break`))

(fn `UserConstructionScript`)